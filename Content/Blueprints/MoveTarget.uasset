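; MoveTarget is a damageable target actor that moves along its local X axis and awards score to the player who destroys it.
; Tick applies the DirentionX offset only while the GameState has exactly two players.
; AnyDamage subtracts floored damage from Health; at zero or below, the server increments the instigator's MyPlayerState score and destroys the actor after a short delay.
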(event `self.ReceiveTick`
  (params (DeltaSeconds :type "Float (single-precision)"))
  (bind _returnvalue (`GameplayStatics.GetGameState`))
  ;[1 1 1] 移动
  (`/Engine/EditorBlueprintResources/StandardMacros.IsValid` _returnvalue
    (:`Is Valid`
      (if (== (`KismetArrayLibrary.Array_Length` (`GameState.PlayerArray` _returnvalue)) 2)
        (`self.K2_AddActorLocalTransform` (`KismetMathLibrary.MakeTransform` (`KismetMathLibrary.MakeVector` (`self.DirentionX`)) (struct) (1.0 1.0 1.0)))))))

(event `self.ReceiveAnyDamage`
  (params (Damage :type "Float (single-precision)") (DamageType :type "DamageType Object Reference") (InstigatedBy :type "Controller Object Reference") (DamageCauser :type "Actor Object Reference"))
  ;[1 1 1] 击中后
  (set `self.Health` (- (`self.Health`) (`KismetMathLibrary.FFloor` Damage)))
  (if (<= (`self.Health`) 0)
    (`/Engine/EditorBlueprintResources/ActorMacros.Switch Has Authority`
      (:`Authority`
        (bind _asmy_player_state (cast `/Game/Blueprints/MyPlayerState` (`Controller.PlayerState` InstigatedBy)))
        (`/Game/Blueprints/MyPlayerState.IncrementScore` _asmy_player_state)
        (`self.DestroySelf`)))))

(event `DestroySelf`
  ;[1 1 1] 击中后
  (`KismetSystemLibrary.Delay` 0.2)
  (`self.K2_DestroyActor`))

(fn `UserConstructionScript`)